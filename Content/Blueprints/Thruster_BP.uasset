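; Thruster actor that launches the player's ball pawn along the thruster's up vector when it hits the thruster mesh.
; The hit applies a velocity-change impulse scaled by ThrusterForce, ignoring the ball's mass, and plays a 2D sound.
; A ThrusterUp timeline offsets the mesh from its BeginPlay location along that vector, with a delayed Reverse triggered from its Update pin to retract it.
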(event OnComponentHit(Thruster)
  (params (HitComponent :type Primitive%20Component%20Object%20Reference) (OtherActor :type Actor%20Object%20Reference) (OtherComp :type Primitive%20Component%20Object%20Reference) (NormalImpulse :type Vector :default "0, 0, 0") (Hit :type Hit%20Result%20Structure%20%28by%20ref%29))
  ;[1 1 1] Thruster Up
  (bind _asball_pawn_bp (Utilities|Casting|CastToBallPawn_BP OtherActor))
  (Physics|AddImpulse (Variables|/Game/Blueprints/BallPawn_BP.BallPawn_BP_C|GetBallMesh _asball_pawn_bp) (* (Math|Vector|GetUpVector (Variables|Default|GetThruster)) (Variables|Default|GetThrusterForce)) "None" true)
  ;[1 1 1] Thruster Animation
  (Audio|PlaySound2D "/Game/Retro_8Bit_Sounds/Collectables/Cues/retro_collect_pickup_item_04_Cue.retro_collect_pickup_item_04_Cue" 1.0 1.0 0.0 0 0)
  (bind _upthrust (Timeline|ThrusterUp Play)
    (:Update
      (Transformation|SetWorldLocation (Variables|Default|GetThruster) (+ (Variables|Default|GetInitialButtonLocation) (* (Math|Vector|GetUpVector (Variables|Default|GetThruster)) _upthrust)) false false)
      (Utilities|FlowControl|Delay 1.0)
      (Timeline|ThrusterUp Reverse))))

(event EventBeginPlay
  (Variables|Default|SetInitialButtonLocation (Transformation|GetWorldLocation (Variables|Default|GetThruster))))

(event Collision|EventActorBeginOverlap
  (params (OtherActor :type Actor%20Object%20Reference)))

(event EventTick
  (params (DeltaSeconds :type Float%20%28single-precision%29)))

(fn ConstructionScript)