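; Game mode for the rolling ball game that restarts play after the player's ball dies.
; On BeginPlay it casts the first player's pawn to BallPawn_BP and caches the reference.
; Tick polls the pawn's IsAlive flag and, once it is false, waits through a short Delay before opening CurrentLevel by name, so respawn is a level load.
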(event EventTick
  (params (DeltaSeconds :type Float%20%28single-precision%29))
  (bind _reftoballpawn (Variables|Default|GetRefToBallPawn))
  ;[1 1 1] Respawn Player Upon Death
  (Utilities|IsValid _reftoballpawn
    (:Is%20Valid
      (if (not (Variables|/Game/Blueprints/BallPawn_BP.BallPawn_BP_C|GetIsAlive _reftoballpawn))
        (Utilities|FlowControl|Delay 2.0)
        (Game|OpenLevel(byName) (Variables|Default|GetCurrentLevel))))))

(event EventBeginPlay
  (bind _output_get (Variables|Default|SetPlayer (Game|Player|GetPlayerPawn 0)))
  (bind _asball_pawn_bp (Utilities|Casting|CastToBallPawn_BP _output_get))
  (Variables|Default|SetRefToBallPawn _asball_pawn_bp))

(fn ConstructionScript)