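; BallPawn_BP is a physics-driven rolling ball pawn that the player rolls and jumps, with a running score.
; Movement axes apply mass-independent torque to BallMesh, and jumping adds a velocity-change vertical impulse with a sound.
; A CanJump flag blocks repeat jumps until any Hit event re-arms it, playing an impact sound if it was unset.
; IncrementScore adds a passed amount to Score.
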(event EventBeginPlay)

(event Collision|EventActorBeginOverlap
  (params (OtherActor :type Actor%20Object%20Reference)))

(event EventTick
  (params (DeltaSeconds :type Float%20%28single-precision%29)))

(event Collision|EventHit
  (params (MyComp :type Primitive%20Component%20Object%20Reference) (Other :type Actor%20Object%20Reference) (OtherComp :type Primitive%20Component%20Object%20Reference) (bSelfMoved :type Boolean) (HitLocation :type Vector :default "0, 0, 0") (HitNormal :type Vector :default "0, 0, 0") (NormalImpulse :type Vector :default "0, 0, 0") (Hit :type Hit%20Result%20Structure%20%28by%20ref%29))
  ;[1 1 1] Jumping Movement
  (if (Variables|Default|GetCanJump)
    _
    (else
      (Audio|PlaySound2D "/Game/Retro_8Bit_Sounds/Impacts/Cues/retro_impact_hit_11_Cue.retro_impact_hit_11_Cue" 1.0 1.0 0.0 0 0)))
  (Variables|Default|SetCanJump true))

(event Input|ActionEvents|InputActionJump
  (params (Key :type Key%20Structure :default "None"))
  ;[1 1 1] Jumping Movement
  (:Pressed
    (if (Variables|Default|GetCanJump)
      (Physics|AddImpulse (Variables|Default|GetBallMesh) (Math|Vector|MakeVector 0.0 0.0 (Variables|Default|GetJumpForce)) "None" true)
      (Variables|Default|SetCanJump false)
      (Audio|PlaySound2D "/Game/Retro_8Bit_Sounds/Jumping/Cues/retro_jump_bounce_12_Cue.retro_jump_bounce_12_Cue" 1.0 1.0 0.0 0 0))))

(event Input|AxisEvents|InputAxisMoveForward
  (params (AxisValue :type Float%20%28single-precision%29))
  ;[1 1 1] Forward/Backward Movement
  (Class|PrimitiveComponent|AddTorqueinDegrees (Variables|Default|GetBallMesh) (Math|Vector|MakeVector 0.0 (* AxisValue (Variables|Default|GetTorque)) 0.0) "None" true))

(event Input|AxisEvents|InputAxisMoveRight
  (params (AxisValue :type Float%20%28single-precision%29))
  ;[1 1 1] Left/Right Movement
  (Class|PrimitiveComponent|AddTorqueinDegrees (Variables|Default|GetBallMesh) (Math|Vector|MakeVector (* AxisValue (Variables|Default|GetTorque) -1.0) 0.0 0.0) "None" true))

(fn ConstructionScript)

(fn IncrementScore
  (params (InScore :type Integer))
  (Variables|Default|SetScore (+ InScore (Variables|Default|GetScore))))