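; Health pickup Blueprint that configures an inherited pickup for its health variant.
; On BeginPlay it sets the damage amount, pickup sound and particle, zeroes the score points and turns off the number widget, then calls the parent BeginPlay.
; The file adds no overlap, tick or construction logic of its own, leaving pickup behavior to the parent class.
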(event EventBeginPlay
  (Variables|Default|SetDamage 20)
  (Variables|Default|SetOnPickupSound "/Game/Retro_8Bit_Sounds/Collectables/Cues/retro_collect_pickup_item_06_Cue.retro_collect_pickup_item_06_Cue")
  (Variables|Default|SetOnPickupParticle "/Game/InfinityBladeEffects/Effects/FX_Ability/Heal/P_Health_Pickup_01.P_Health_Pickup_01")
  (Variables|Default|SetPoints 0)
  (Variables|Default|SetUseNumberWidget false)
  (|CallParentFunction))

(event Collision|EventActorBeginOverlap
  (params (OtherActor :type Actor%20Object%20Reference))
  (|CallParentFunction OtherActor) ; This node is disabled and will not be called.\nDrag off pins to build functionality.
)

(event EventTick
  (params (DeltaSeconds :type Float%20%28single-precision%29))
  (|CallParentFunction DeltaSeconds) ; This node is disabled and will not be called.\nDrag off pins to build functionality.
)

(fn ConstructionScript
  (|CallParentFunction))