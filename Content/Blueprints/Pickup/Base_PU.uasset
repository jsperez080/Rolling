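; Base pickup actor that awards points to the ball pawn on contact, with a sound and particle effect.
; On start, it passes its point value to a hidden PickupText widget.
; OnPickup either hides the mesh and plays the widget's animation, or destroys the actor immediately, depending on UseNumberWidget.
; The sphere overlap handler also destroys the actor after a short delay, whichever actor overlapped it.
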(event OnComponentBeginOverlap(Sphere)
  (params (OverlappedComponent :type Primitive%20Component%20Object%20Reference) (OtherActor :type Actor%20Object%20Reference) (OtherComp :type Primitive%20Component%20Object%20Reference) (OtherBodyIndex :type Integer) (bFromSweep :type Boolean) (SweepResult :type Hit%20Result%20Structure%20%28by%20ref%29))
  ;[1 1 1] Pickup Interactivity
  (CallFunction|OnPickup OtherActor)
  (Utilities|FlowControl|Delay 1.0)
  (Actor|DestroyActor))

(event EventBeginPlay
  (bind _pickuptext (Variables|Default|GetPickupText))
  (Rendering|SetVisibility _pickuptext false false)
  (bind _aspickup_text (Utilities|Casting|CastToPickupText (UserInterface|GetUserWidgetObject _pickuptext)))
  (Variables|/Game/Blueprints/Pickup/PickupText.PickupText_C|SetScoreValue _aspickup_text (Variables|Default|GetPoints)))

(event Collision|EventActorBeginOverlap
  (params (OtherActor :type Actor%20Object%20Reference)))

(event EventTick
  (params (DeltaSeconds :type Float%20%28single-precision%29)))

(fn ConstructionScript)

(fn OnPickup
  (params (OtherActor :type Object%20Object%20Reference))
  (bind _asball_pawn_bp (Utilities|Casting|CastToBallPawn_BP OtherActor))
  (Default|IncrementScore _asball_pawn_bp (Variables|Default|GetPoints))
  (Audio|PlaySound2D (Variables|Default|GetOnPickupSound) 1.0 1.0 0.0 0 0)
  (Effects|SpawnEmitteratLocation (Variables|Default|GetOnPickupParticle) (Transformation|GetActorLocation))
  (if (Variables|Default|GetUseNumberWidget)
    (Utilities|FlowControl|Sequence
      (:then_0
        (Rendering|SetVisibility (Variables|Default|GetStaticMesh) false false))
      (:then_1
        (Rendering|SetVisibility (Variables|Default|GetPickupText) true false)
        (bind _aspickup_text (Utilities|Casting|CastToPickupText (UserInterface|GetUserWidgetObject (Variables|Default|GetPickupText))))
        (UserInterface|Animation|PlayAnimation _aspickup_text (Variables|/Game/Blueprints/Pickup/PickupText.PickupText_C|GetPickupAnimation _aspickup_text) 0.0 1 "Forward" 1.0 false)))
    (else
      (Actor|DestroyActor))))