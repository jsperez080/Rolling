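; Explosive pickup hazard that blasts the player's ball on contact.
; BeginPlay configures the parent pickup with explosion sound and particle, no points, a negative Damage value and no number widget.
; On pickup it applies a radial impulse to the BallPawn_BP mesh from just below itself, then runs the parent logic.
; It binds to the player pawn's DestroyHazards event to destroy itself when that fires.
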(event Custom|DestroySelf
  (Actor|DestroyActor))

(event EventBeginPlay
  (Utilities|FlowControl|Sequence
    (:then_0
      (Variables|Default|SetUseNumberWidget false))
    (:then_1
      (Variables|Default|SetOnPickupSound "/Game/StarterContent/Audio/Explosion01.Explosion01"))
    (:then_2
      (Variables|Default|SetOnPickupParticle "/Game/StarterContent/Particles/P_Explosion.P_Explosion"))
    (:then_3
      (Variables|Default|SetPoints 0))
    (:then_4
      (Variables|Default|SetDamage -50))
    (:then_5
      (|CallParentFunction)
      (EventDispatchers|BindEventtoDestroyHazards (.AsBall%20Pawn%20BP (Utilities|Casting|CastToBallPawn_BP (Game|Player|GetPlayerPawn 0))) (delegate Custom|DestroySelf)))))

(event Collision|EventActorBeginOverlap
  (params (OtherActor :type Actor%20Object%20Reference))
  (|CallParentFunction OtherActor) ; This node is disabled and will not be called.\nDrag off pins to build functionality.
)

(event EventTick
  (params (DeltaSeconds :type Float%20%28single-precision%29))
  (|CallParentFunction DeltaSeconds) ; This node is disabled and will not be called.\nDrag off pins to build functionality.
)

(event EventOnPickup
  (params (OtherActor :type Object%20Object%20Reference))
  (bind _returnvalue (Transformation|GetActorLocation))
  (bind (_x _y _z) (Math|Vector|BreakVector _returnvalue))
  (bind _asball_pawn_bp (Utilities|Casting|CastToBallPawn_BP OtherActor))
  (Physics|AddRadialImpulse (Variables|/Game/Blueprints/BallPawn_BP.BallPawn_BP_C|GetBallMesh _asball_pawn_bp) (Math|Vector|MakeVector _x _y (+ _z -75.0)) 5e+02 1e+03 "RIF_Constant" true)
  (|CallParentFunction OtherActor))

(fn ConstructionScript
  (|CallParentFunction))